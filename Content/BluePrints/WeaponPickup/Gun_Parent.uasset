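; Base gun Blueprint for first-person weapons, with arms and gun components and projectile firing.
; The construction script snaps the gun to the arms' GripPoint socket.
; FireBullet casts the parent actor to FirstPersonCharacter, spawns a projectile at the barrel using the camera's rotation, and plays the arms' fire montage.
; StartShooting and StopShooting only toggle a firing flag; nothing here reads it or calls FireBullet.
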(event `StartShooting`
  (set `self.IsFirring` true))

(event `StopShooting`
  (set `self.IsFirring` false))

(fn `FireBullet`
  (bind _asfirst_person_character (cast `/Game/FirstPersonBP/Blueprints/FirstPersonCharacter` (`self.GetParentActor`)))
  (`|SpawnActorFromClass` "/Game/FirstPersonBP/Blueprints/FirstPersonProjectile.FirstPersonProjectile_C" (`KismetMathLibrary.MakeTransform` (`SceneComponent.K2_GetComponentLocation` (`self.Barrel_reference`)) (`SceneComponent.K2_GetComponentRotation` (`/Game/FirstPersonBP/Blueprints/FirstPersonCharacter.FirstPersonCamera` _asfirst_person_character))) "Undefined" "OverrideRootScale" null null)
  (`AnimInstance.Montage_Play` (`SkeletalMeshComponent.GetAnimInstance` (`self.Arms`)) "/Game/FirstPerson/Animations/FirstPersonFire_Montage.FirstPersonFire_Montage" 1.0 "MontageLength" 0.0 true))

(fn `UserConstructionScript`
  (`SceneComponent.K2_AttachToComponent` (`self.Guns`) (`self.Arms`) "GripPoint" "SnapToTarget" "SnapToTarget" "SnapToTarget" true))